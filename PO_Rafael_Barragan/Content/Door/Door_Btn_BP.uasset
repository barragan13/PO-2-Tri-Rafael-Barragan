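; Button door Blueprint that lets a nearby player toggle a door with the Interact input.
; Entering the Box trigger shows an Interact widget and enables input; leaving disables input and removes all widgets.
; Each press flips the Open boolean and plays or reverses the Open timeline, which lerps the Child Actor's relative yaw through a half turn.
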(event `InputAction|Interact`
  (params (Key :type "Key Structure"))
  ;[1 1 1] Funcionameto da porta com botão
  ;;[1 1 1] Checa se quando o input for acionado a porta está aberta
  (:`Pressed`
    (if (`self.Open?`)
      (set `self.Open?` false)
      ;;[1 1 1] Aciona a animação de rotação sobre o eixo do 'Child Actor'
      (bind (_direction _newtrack_0) (`Timeline|Open` :!label _label)
        (:`Update`
          (`SceneComponent.K2_SetRelativeRotation` (`self.ChildActor`) (`KismetMathLibrary.MakeRotator` 0.0 0.0 (`KismetMathLibrary.Lerp` 0.0 180.0 _newtrack_0)) false false)))
      (else
        (set `self.Open?` true)
        (goto _label :!via `Reverse`)))))

(event `self.Box.OnComponentBeginOverlap`
  (params (OverlappedComponent :type "PrimitiveComponent Object Reference") (OtherActor :type "Actor Object Reference") (OtherComp :type "PrimitiveComponent Object Reference") (OtherBodyIndex :type Integer) (bFromSweep :type Boolean) (SweepResult :type "HitResult Structure (by ref)"))
  ;[1 0.991 0.7292] Adiciona a interface de interação na tela quando o jogador se aproxima da box
  (bind _returnvalue (`|CreateWidget` "/Game/Door/Interface/Interact.Interact_C"))
  (`UserWidget.AddToViewport` _returnvalue 0)
  (`self.EnableInput` (`GameplayStatics.GetPlayerController` 0)))

(event `self.Box.OnComponentEndOverlap`
  (params (OverlappedComponent :type "PrimitiveComponent Object Reference") (OtherActor :type "Actor Object Reference") (OtherComp :type "PrimitiveComponent Object Reference") (OtherBodyIndex :type Integer))
  ;[1 0.991 0.7292] Adiciona a interface de interação na tela quando o jogador se aproxima da box
  (`self.DisableInput` (`GameplayStatics.GetPlayerController` 0))
  (`WidgetLayoutLibrary.RemoveAllWidgets`))

(fn `UserConstructionScript`)