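; Hologram actor that lets the player show or hide its sphere while inside a trigger box.
; Entering the box adds a ShowHide widget to the viewport and enables input for player controller 0.
; The Destroy input action toggles the sphere's visibility, tracked by the WorldShow flag, without destroying anything.
; Leaving the box disables input and removes all widgets, with no filter on the overlapping actor in either event.
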(event `InputAction|Destroy`
  (params (Key :type "Key Structure"))
  (bind _sphere (`self.Sphere`))
  (:`Pressed`
    (if (`self.World show?`)
      (`SceneComponent.SetVisibility` _sphere false false)
      (set `self.World show?` false)
      (else
        (`SceneComponent.SetVisibility` _sphere true false)
        (set `self.World show?` true)))))

(event `self.Box.OnComponentBeginOverlap`
  (params (OverlappedComponent :type "PrimitiveComponent Object Reference") (OtherActor :type "Actor Object Reference") (OtherComp :type "PrimitiveComponent Object Reference") (OtherBodyIndex :type Integer) (bFromSweep :type Boolean) (SweepResult :type "HitResult Structure (by ref)"))
  (bind _returnvalue (`|CreateWidget` "/Game/Shader/Hologram/ShowHide.ShowHide_C"))
  (`UserWidget.AddToViewport` _returnvalue 0)
  (`self.EnableInput` (`GameplayStatics.GetPlayerController` 0)))

(event `self.Box.OnComponentEndOverlap`
  (params (OverlappedComponent :type "PrimitiveComponent Object Reference") (OtherActor :type "Actor Object Reference") (OtherComp :type "PrimitiveComponent Object Reference") (OtherBodyIndex :type Integer))
  (`self.DisableInput` (`GameplayStatics.GetPlayerController` 0))
  (`WidgetLayoutLibrary.RemoveAllWidgets`))

(fn `UserConstructionScript`)